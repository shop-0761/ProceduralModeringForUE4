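; BP_Tubular builds a procedural tube mesh along a spline, with configurable radius, radial and tubular segments, and an optional closed loop.
; DrawMesh seeds a normal from the start tangent's smallest component, then computes Frenet frames along the spline.
; GenerateSegment adds a ring of vertices, normals and tangents per frame.
; DrawMesh then adds UVs, stitches rings into triangles and creates the mesh section.
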(event EventBeginPlay)

(event Collision|EventActorBeginOverlap
  (params (OtherActor :type Actor%20Object%20Reference)))

(event EventTick
  (params (DeltaSeconds :type Float%20%28single-precision%29)))

(event EventClearArrays
  (Utilities|Array|Clear (Variables|Default|GetVeticies))
  (Utilities|Array|Clear (Variables|Default|GetNormals))
  (Utilities|Array|Clear (Variables|Default|GetUV))
  (Utilities|Array|Clear (Variables|Default|GetTriangles))
  (Utilities|Array|Clear (Variables|Default|GetTangents)))

(fn ConstructionScript
  (|CallParentFunction))

(fn DrawMesh
  (bind _spline (Variables|Default|GetSpline))
  (bind _tubularsegments (Variables|Default|GetTubularSegments))
  (bind _radialsegments (Variables|Default|GetRadialSegments))
  (bind _returnvalue (Spline|GetTangentatSplinePoint _spline 0 "Local"))
  (bind _returnvalue_2 (+ _radialsegments 2))
  (bind _returnvalue_3 (Math|Vector|Normalize _returnvalue))
  (bind (_x _y _z) (Math|Vector|BreakVector _returnvalue_3))
  (bind _returnvalue_4 (Math|Float|Min(Float) _x _y _z))
  (CallFunction|ClearArrays)
  (if (Math|Float|NearlyEqual(Float) _x _returnvalue_4 1e-06)
    (LocalVariables|Setnormal "1.000000, 0, 0")
    (elif (Math|Float|NearlyEqual(Float) _y _returnvalue_4 1e-06)
      (LocalVariables|Setnormal "0,1.000000, 0")
      (else
        (LocalVariables|Setnormal "0, 0,1.000000"))))
  (LocalVariables|Setnormal (Math|Vector|CrossProduct _returnvalue_3 (Math|Vector|CrossProduct _returnvalue_3 (LocalVariables|Getnormal))))
  (LocalVariables|Setbinormal (Math|Vector|CrossProduct _returnvalue_3 (Math|Vector|CrossProduct _returnvalue_3 (Math|Vector|CrossProduct _returnvalue_3 (LocalVariables|Getnormal)))))
  (bind _frames (CallFunction|ComputeFrenetFrames (Variables|Default|GetSpline) (Variables|Default|GetTubularSegments) (LocalVariables|Getnormal) (LocalVariables|Getbinormal) (Variables|Default|GetClosed)))
  (for _index (range 0 _tubularsegments)
    (CallFunction|GenerateSegment _frames (Variables|Default|GetVeticies) (Variables|Default|GetNormals) (Variables|Default|GetTangents) _index))
  (CallFunction|GenerateSegment _frames (Variables|Default|GetVeticies) (Variables|Default|GetNormals) (Variables|Default|GetTangents) (Math|Integer|SelectInt (Variables|Default|GetTubularSegments) 0 (not (Variables|Default|GetClosed))))
  (for _index_2 (range 0 (+ _tubularsegments 1))
    (for _index_3 (range 0 (+ (Variables|Default|GetRadialSegments) 1))
      (Utilities|Array|Add (Variables|Default|GetUV) (Math|Vector2D|MakeVector2D (/ (Math|Conversions|ToFloat(Integer) _index_3) (Math|Conversions|ToFloat(Integer) (Variables|Default|GetRadialSegments))) (/ (Math|Conversions|ToFloat(Integer) _index_2) (Math|Conversions|ToFloat(Integer) (Variables|Default|GetTubularSegments)))))))
  (for _index_4 (range 1 (Variables|Default|GetTubularSegments))
    (for _index_5 (range 1 (+ (Variables|Default|GetRadialSegments) 1))
      (bind _output_get (LocalVariables|Seta (+ (- _index_5 1) (* (- _index_4 1) _returnvalue_2))))
      (bind _output_get_2 (LocalVariables|Setb (+ (- _index_5 1) (* _returnvalue_2 _index_4))))
      (bind _output_get_3 (LocalVariables|Setc (+ _index_5 (* _returnvalue_2 _index_4))))
      (bind _output_get_4 (LocalVariables|Setd (+ _index_5 (* (- _index_4 1) _returnvalue_2))))
      (Utilities|Array|AppendArray (Variables|Default|GetTriangles) (Utilities|Array|MakeArray _output_get _output_get_4 _output_get_2 _output_get_2 _output_get_4 _output_get_3))))
  (Class|ProceduralMeshComponent|CreateMeshSectionLinearColor (Variables|Default|GetProceduralMesh) 0 (Variables|Default|GetVeticies) (Variables|Default|GetTriangles) (Variables|Default|GetNormals) (Variables|Default|GetUV) 0 (Variables|Default|GetTangents) false)
  (return true))

(fn GenerateSegment
  (params (Frames :type Array%20of%20Frenet%20Frame%20Structures) (Vertices :type Array%20of%20Vectors) (Normals :type Array%20of%20Vectors) (Tangents :type Array%20of%20Proc%20Mesh%20Tangent%20Structures) (Index :type Integer))
  (bind _output (Utilities|Array|Get(acopy) Frames Index))
  (bind _radialsegments (Variables|Default|GetRadialSegments))
  (for _index (range 0 (+ _radialsegments 1))
    (Utilities|Array|Add Vertices (+ (* (Math|Vector|Normalize (+ (* (.normal _output) (Math|Trig|Cos(Radians) (* (/ (Math|Conversions|ToFloat(Integer) _index) (Math|Conversions|ToFloat(Integer) _radialsegments)) (* (Math|Trig|GetPI) 2.0)))) (* (.binormal _output) (Math|Trig|Sin(Radians) (* (/ (Math|Conversions|ToFloat(Integer) _index) (Math|Conversions|ToFloat(Integer) _radialsegments)) (* (Math|Trig|GetPI) 2.0)))))) (Variables|Default|GetRadius)) (Spline|GetLocationatDistanceAlongSpline (Variables|Default|GetSpline) (* (/ (Math|Conversions|ToFloat(Integer) Index) (Math|Conversions|ToFloat(Integer) (Variables|Default|GetTubularSegments))) (Spline|GetSplineLength (Variables|Default|GetSpline))) "Local")))
    (Utilities|Array|Add Normals (Math|Vector|Normalize (+ (* (.normal _output) (Math|Trig|Cos(Radians) (* (/ (Math|Conversions|ToFloat(Integer) _index) (Math|Conversions|ToFloat(Integer) _radialsegments)) (* (Math|Trig|GetPI) 2.0)))) (* (.binormal _output) (Math|Trig|Sin(Radians) (* (/ (Math|Conversions|ToFloat(Integer) _index) (Math|Conversions|ToFloat(Integer) _radialsegments)) (* (Math|Trig|GetPI) 2.0)))))))
    (Utilities|Array|Add Tangents (.tangent _output))))