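; BP_Plane is a procedural mesh Blueprint that generates a segmented, flat plane sized by width, height and segment counts.
; DrawMesh fills grid vertices, UVs, up-facing normals and triangle indices, then creates the ProceduralMesh section.
; While building triangles, it sets vertex Z from DepthFunc, which returns zero here and acts as a height hook over normalized grid coordinates.
; The construction script only calls its parent.
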(fn ConstructionScript
  (|CallParentFunction))

(fn DepthFunc
  (params (rx :type Float%20%28single-precision%29) (ry :type Float%20%28single-precision%29))
  (return 0.0))

(fn DrawMesh
  (bind _widthsegments (Variables|Default|GetWidthSegments))
  (bind _widthsegments_2 (Variables|Default|GetWidthSegments))
  (bind _veticies (Variables|Default|GetVeticies))
  (CallFunction|ClearArrays)
  (LocalVariables|Setwinv (/ 1.0 (Math|Conversions|ToFloat(Integer) (- (Variables|Default|GetWidthSegments) 1))))
  (LocalVariables|Sethinv (/ 1.0 (Math|Conversions|ToFloat(Integer) (- (Variables|Default|GetHeightSegments) 1))))
  (for _index (range 0 (Variables|Default|GetHeightSegments))
    (LocalVariables|Setry (* _index (LocalVariables|Gethinv)))
    (for _index_2 (range 0 (Variables|Default|GetWidthSegments))
      (LocalVariables|Setrx (* _index_2 (LocalVariables|Getwinv)))
      (Utilities|Array|Add (Variables|Default|GetVeticies) (Math|Vector|MakeVector (* (- (LocalVariables|Getrx) 0.5) (Variables|Default|GetWidth)) (* (- 0.5 (LocalVariables|Getry)) (Variables|Default|GetHeight)) 0.0))
      (Utilities|Array|Add (Variables|Default|GetUV) (Math|Vector2D|MakeVector2D (LocalVariables|Getrx) (LocalVariables|Getry)))
      (Utilities|Array|Add (Variables|Default|GetNormals) "0,0.000000,1.000000")))
  (for _index_3 (range 0 (- (Variables|Default|GetHeightSegments) 1))
    (LocalVariables|Setry (* _index_3 (LocalVariables|Gethinv)))
    (for _index_4 (range 0 (- _widthsegments 1))
      (LocalVariables|Setrx (* _index_4 (LocalVariables|Getwinv)))
      (LocalVariables|Setindex (+ _index_4 (* _index_3 (+ _widthsegments 1))))
      (LocalVariables|Seta (LocalVariables|Getindex))
      (LocalVariables|Setb (+ (LocalVariables|Getindex) 1))
      (LocalVariables|Setc (+ (LocalVariables|Getindex) _widthsegments_2 1))
      (LocalVariables|Setd (+ (LocalVariables|Getindex) _widthsegments_2 2))
      (Utilities|Array|AppendArray (Variables|Default|GetTriangles) (Utilities|Array|MakeArray (LocalVariables|Geta) (LocalVariables|Getb) (LocalVariables|Getc) (LocalVariables|Getc) (LocalVariables|Getb) (LocalVariables|Getd)))
      (Utilities|Array|SetArrayElem _veticies (LocalVariables|Getindex) (Math|Vector|MakeVector (.x (Utilities|Array|Get(acopy) _veticies (LocalVariables|Getindex))) (.y (Utilities|Array|Get(acopy) _veticies (LocalVariables|Getindex))) (CallFunction|DepthFunc (LocalVariables|Getrx) (LocalVariables|Getry))))))
  (Class|ProceduralMeshComponent|CreateMeshSectionLinearColor (Variables|Default|GetProceduralMesh) 0 (Variables|Default|GetVeticies) (Variables|Default|GetTriangles) (Variables|Default|GetNormals) (Variables|Default|GetUV) 0 0 false)
  (return true))