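; BP_TreeBranch is a procedural tree branch actor that recursively spawns child branches to grow a tree skeleton.
; On BeginPlay it randomly rotates its growth direction and builds a bent spline, sampling Frenet frames into segments with tapering radius.
; Until Generation reaches zero, it spawns children from segments along its outer half, passing on frame, radius, attenuated length and shared Data with an incremented seed.
; Last-generation branches taper to zero radius.
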(event EventBeginPlay
  (CallFunction|Constructor))

(fn ConstructionScript)

(fn BuildSegments
  (params (Data :type BPC%20Tree%20Data%20Object%20Reference) (FromRadius :type Float%20%28single-precision%29) (ToRadius :type Float%20%28single-precision%29) (Normal :type Vector) (Binormal :type Vector))
  (bind _returnvalue (Default|GetRandomBendDegree Data))
  (bind _from (Variables|Default|GetFrom))
  (bind _to (Variables|Default|GetTo))
  (bind _spline (Variables|Default|GetSpline))
  (Utilities|Array|Clear (LocalVariables|Get_Segments))
  (Spline|ClearSplinePoints (Variables|Default|GetSpline) true)
  (LocalVariables|Set_Length (Math|Vector|VectorLength (- (Variables|Default|GetTo) (Variables|Default|GetFrom))))
  (LocalVariables|Set_Bend (* (+ (* Normal _returnvalue) (* Binormal _returnvalue)) (LocalVariables|Get_Length)))
  (Spline|SetSplinePoints (Variables|Default|GetSpline) (Utilities|Array|MakeArray _from (+ (LocalVariables|Get_Bend) (Math|Vector|Lerp(Vector) _from _to 0.25)) (+ (LocalVariables|Get_Bend) (Math|Vector|Lerp(Vector) _from _to 0.75)) _to) "Local" true)
  (bind _frames (CallFunction|ComputeFrenetFrames (Variables|Default|GetSpline) (Variables|/Game/BluePrints/ProceduralModering/BPC_TreeData.BPC_TreeData_C|GetHeightSegments (Variables|Default|GetData)) Normal Binormal false))
  (for (_array_element _array_index) _frames
    (Utilities|Array|Add (LocalVariables|Get_Segments) (Utilities|Struct|MakeTreeSegment _array_element (Spline|GetLocationatDistanceAlongSpline _spline (* (/ (Math|Conversions|ToFloat(Integer) _array_index) (Math|Conversions|ToFloat(Integer) (- (Utilities|Array|Length _frames) 1))) (Spline|GetSplineLength _spline)) "Local") (Math|Float|Lerp FromRadius ToRadius (/ (Math|Conversions|ToFloat(Integer) _array_index) (Math|Conversions|ToFloat(Integer) (- (Utilities|Array|Length _frames) 1)))))))
  (return (LocalVariables|Get_Segments)))

(fn Constructor
  (bind _data (Variables|Default|GetData))
  (bind _data_2 (Variables|Default|GetData))
  (Variables|Default|SetToRadius (Math|Float|SelectFloat 0.0 (* (Variables|Default|GetFromRadius) (Variables|/Game/BluePrints/ProceduralModering/BPC_TreeData.BPC_TreeData_C|GetRadiusAttenuation _data_2)) (== (Variables|Default|GetGeneration) 0)))
  (LocalVariables|Set_Scale (Math|Float|Lerp 1.0 (Variables|/Game/BluePrints/ProceduralModering/BPC_TreeData.BPC_TreeData_C|GetGrowAngleScale _data_2) (- 1.0 (/ (Math|Conversions|ToFloat(Integer) (Variables|Default|GetGeneration)) (Math|Conversions|ToFloat(Integer) (Variables|Default|GetGenerations))))))
  (LocalVariables|Set_qn (Math|Vector|RotatorfromAxisandAngle (Variables|Default|GetNormal) (* (LocalVariables|Get_Scale) (Default|GetRandomGrowthAngle _data_2))))
  (LocalVariables|Set_qb (Math|Vector|RotatorfromAxisandAngle (Variables|Default|GetBinormal) (* (LocalVariables|Get_Scale) (Default|GetRandomGrowthAngle _data_2))))
  (Variables|Default|SetTo (+ (Variables|Default|GetFrom) (* (Math|Vector|Normalize (Math|Vector|RotateVector (.TangentX (Utilities|Struct|BreakProcMeshTangent (Variables|Default|GetTangent))) (Math|Rotator|CombineRotators (LocalVariables|Get_qn) (LocalVariables|Get_qb)))) (Variables|Default|GetLength))))
  (bind _segments (CallFunction|BuildSegments (Variables|Default|GetData) (Variables|Default|GetFromRadius) (Variables|Default|GetToRadius) (Variables|Default|GetNormal) (Variables|Default|GetBinormal)))
  (bind _output_get (Variables|Default|SetSegments _segments))
  (if (> (Variables|Default|GetGeneration) 0)
    (bind _output_get_2 (LocalVariables|Set_Count (Default|GetRandomBranches (Variables|Default|GetData))))
    (for _index (range 0 (- _output_get_2 1))
      (if (== (LocalVariables|Get_Count) 1)
        (LocalVariables|Set_Ratio 1.0)
        (else
          (LocalVariables|Set_Ratio (Math|Float|Lerp 0.5 1.0 (/ (Math|Conversions|ToFloat(Integer) _index) (Math|Conversions|ToFloat(Integer) (- (LocalVariables|Get_Count) 1)))))))
      (Variables|/Game/BluePrints/ProceduralModering/BPC_TreeData.BPC_TreeData_C|SetRandomSeed _data (+ (Variables|/Game/BluePrints/ProceduralModering/BPC_TreeData.BPC_TreeData_C|GetRandomSeed _data) 1))
      (bind _returnvalue (Game|SpawnActorfromClass "BP_TreeBranch_C" (Transformation|GetActorTransform) "Undefined" 0 (- (Variables|Default|GetGeneration) 1) (Variables|Default|GetGenerations) (.Location (Utilities|Struct|BreakTreeSegment (Utilities|Array|Get(acopy) _output_get (- (Math|Float|Floor (* (- (Utilities|Array|Length _output_get) 1) (LocalVariables|Get_Ratio))) 1)))) (.Tangent (Utilities|Struct|BreakFrenetFrame (.Frame (Utilities|Struct|BreakTreeSegment (Utilities|Array|Get(acopy) _output_get (- (Math|Float|Floor (* (- (Utilities|Array|Length _output_get) 1) (LocalVariables|Get_Ratio))) 1)))))) (.Normal (Utilities|Struct|BreakFrenetFrame (.Frame (Utilities|Struct|BreakTreeSegment (Utilities|Array|Get(acopy) _output_get (- (Math|Float|Floor (* (- (Utilities|Array|Length _output_get) 1) (LocalVariables|Get_Ratio))) 1)))))) (.Binormal (Utilities|Struct|BreakFrenetFrame (.Frame (Utilities|Struct|BreakTreeSegment (Utilities|Array|Get(acopy) _output_get (- (Math|Float|Floor (* (- (Utilities|Array|Length _output_get) 1) (LocalVariables|Get_Ratio))) 1)))))) (* (Variables|Default|GetLength) (Math|Float|Lerp 1.0 (Variables|/Game/BluePrints/ProceduralModering/BPC_TreeData.BPC_TreeData_C|GetLengthAttenuation (Variables|Default|GetData)) (LocalVariables|Get_Ratio))) (.Radius (Utilities|Struct|BreakTreeSegment (Utilities|Array|Get(acopy) _output_get (- (Math|Float|Floor (* (- (Utilities|Array|Length _output_get) 1) (LocalVariables|Get_Ratio))) 1)))) (+ (Variables|Default|GetLength) (Variables|Default|GetOffset)) (Variables|Default|GetData)))
      (Utilities|Array|Add (Variables|Default|GetBranchChildren) _returnvalue))))