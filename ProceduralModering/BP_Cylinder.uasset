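; Procedural cylinder Blueprint whose DrawMesh builds a mesh section from Height, Radius and Segments, centred on the local origin.
; GenerateCap emits paired top and bottom ring vertices with UVs and radial or vertical normals, which DrawMesh stitches into side quads.
; Despite its name, OpenEnded set to true adds both caps: duplicated rings fanned to centre vertices using a custom stepped-loop macro.
; The construction script and events here never call DrawMesh.
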(event EventBeginPlay)

(event Collision|EventActorBeginOverlap
  (params (OtherActor :type Actor%20Object%20Reference)))

(event EventTick
  (params (DeltaSeconds :type Float%20%28single-precision%29)))

(fn ConstructionScript
  (|CallParentFunction))

(fn GenerateCap
  (params (segments :type Integer) (top :type Float%20%28single-precision%29) (bottom :type Float%20%28single-precision%29) (radius :type Float%20%28single-precision%29) (Vercies :type Array%20of%20Vectors) (uvs :type Array%20of%20Vector%202D%20Structures) (normals :type Array%20of%20Vectors) (side :type Boolean))
  (for _index (range 0 segments)
    (bind _output_get (LocalVariables|Setratio (/ (Math|Conversions|ToFloat(Integer) _index) (Math|Conversions|ToFloat(Integer) (- segments 1)))))
    ;[1 1 1] top
    (Utilities|Array|Add Vercies (Math|Vector|MakeVector (* radius (Math|Trig|Cos(Radians) (* _output_get (* (Math|Trig|GetPI) 2.0)))) (* radius (Math|Trig|Sin(Radians) (* _output_get (* (Math|Trig|GetPI) 2.0)))) top))
    (Utilities|Array|Add uvs (Math|Vector2D|MakeVector2D (LocalVariables|Getratio) 1.0))
    ;[1 1 1] bottom
    (Utilities|Array|Add Vercies (Math|Vector|MakeVector (* radius (Math|Trig|Cos(Radians) (* _output_get (* (Math|Trig|GetPI) 2.0)))) (* radius (Math|Trig|Sin(Radians) (* _output_get (* (Math|Trig|GetPI) 2.0)))) bottom))
    (Utilities|Array|Add uvs (Math|Vector2D|MakeVector2D (LocalVariables|Getratio) 0.0))
    (if side
      (Utilities|Array|Add normals (Math|Vector|MakeVector (Math|Trig|Cos(Radians) (* _output_get (* (Math|Trig|GetPI) 2.0))) (Math|Trig|Sin(Radians) (* _output_get (* (Math|Trig|GetPI) 2.0))) 0.0))
      (Utilities|Array|Add normals (Math|Vector|MakeVector (Math|Trig|Cos(Radians) (* _output_get (* (Math|Trig|GetPI) 2.0))) (Math|Trig|Sin(Radians) (* _output_get (* (Math|Trig|GetPI) 2.0))) 0.0))
      (else
        (Utilities|Array|Add normals "0,0,1.000000")
        (Utilities|Array|Add normals "0,0,-1.000000")))))

(fn DrawMesh
  (bind _segments (Variables|Default|GetSegments))
  (bind _veticies (Variables|Default|GetVeticies))
  (bind _height (Variables|Default|GetHeight))
  (bind _returnvalue (Utilities|Array|Length _veticies))
  (bind _returnvalue_2 (+ _segments 1))
  (CallFunction|ClearArrays)
  (LocalVariables|Settop (* _height 0.5))
  (LocalVariables|Setbottom (* _height -1.0 0.5))
  (CallFunction|GenerateCap _returnvalue_2 (LocalVariables|Gettop) (LocalVariables|Getbottom) (Variables|Default|GetRadius) (Variables|Default|GetVeticies) (Variables|Default|GetUV) (Variables|Default|GetNormals) true)
  (LocalVariables|Setlen (* (+ _returnvalue_2 1) 2))
  (for _index (range 0 _segments)
    (bind _output_get (LocalVariables|Setidx (* _index 2)))
    (LocalVariables|Seta _output_get)
    (LocalVariables|Setb (+ _output_get 1))
    (LocalVariables|Setc (Math|Integer|%(Integer) (+ _output_get 2) (LocalVariables|Getlen)))
    (LocalVariables|Setd (Math|Integer|%(Integer) (+ _output_get 3) (LocalVariables|Getlen)))
    (Utilities|Array|AppendArray (Variables|Default|GetTriangles) (Utilities|Array|MakeArray (LocalVariables|Geta) (LocalVariables|Getc) (LocalVariables|Getb) (LocalVariables|Getd) (LocalVariables|Getb) (LocalVariables|Getc))))
  (if (Variables|Default|GetopenEnded)
    (CallFunction|GenerateCap (+ (Variables|Default|GetSegments) 1) (LocalVariables|Gettop) (LocalVariables|Getbottom) (Variables|Default|GetRadius) (Variables|Default|GetVeticies) (Variables|Default|GetUV) (Variables|Default|GetNormals) false)
    ;[1 1 1] top center vertex
    (Utilities|Array|Add (Variables|Default|GetVeticies) (Math|Vector|MakeVector 0.0 0.0 (LocalVariables|Gettop)))
    (Utilities|Array|Add (Variables|Default|GetUV) "(X=0.500000,Y=1.000000)")
    (Utilities|Array|Add (Variables|Default|GetNormals) "0,0,1.000000")
    ;[1 1 1] bottom center vertex
    (Utilities|Array|Add (Variables|Default|GetVeticies) (Math|Vector|MakeVector 0.0 0.0 (LocalVariables|Getbottom)))
    (Utilities|Array|Add (Variables|Default|GetUV) "(X=0.500000,Y=0.000000)")
    (Utilities|Array|Add (Variables|Default|GetNormals) "0,0,-1.000000")
    (LocalVariables|Setit (- _returnvalue 2))
    (LocalVariables|Setib (- _returnvalue 1))
    (LocalVariables|Setoffset (LocalVariables|Getlen))
    (bind _index_2 (Utilities|ForLoopwithSelfCounter 0 (LocalVariables|Getlen) 2)
      (:LoopBody
        (Utilities|Array|AppendArray (Variables|Default|GetTriangles) (Utilities|Array|MakeArray (LocalVariables|Getit) (+ (Math|Integer|%(Integer) (+ _index_2 2) (LocalVariables|Getlen)) (LocalVariables|Getoffset)) (+ _index_2 (LocalVariables|Getoffset)))))
      (:Completed
        (bind _index_3 (Utilities|ForLoopwithSelfCounter 1 (LocalVariables|Getlen) 2)
          (:LoopBody
            (Utilities|Array|AppendArray (Variables|Default|GetTriangles) (Utilities|Array|MakeArray (LocalVariables|Getib) (+ _index_3 (LocalVariables|Getoffset)) (+ (Math|Integer|%(Integer) (+ _index_3 2) (LocalVariables|Getlen)) (LocalVariables|Getoffset)))))
          (:Completed
            (Class|ProceduralMeshComponent|CreateMeshSectionLinearColor (Variables|Default|GetProceduralMesh) 0 (Variables|Default|GetVeticies) (Variables|Default|GetTriangles) (Variables|Default|GetNormals) (Variables|Default|GetUV) 0 0 false :!label _label)
            (return true)))))
    (else
      (goto _label))))