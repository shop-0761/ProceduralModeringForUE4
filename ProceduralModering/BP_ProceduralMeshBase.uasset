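; Base procedural mesh actor with a stub DrawMesh, apparently for child Blueprints to override, and debug visualization of mesh data.
; The construction script calls DrawMesh, then in Debug mode applies a standard, UV or normal material and visualizes the vertex, normal and triangle arrays.
; Index-shaded meshes mark vertices, while arrows show normals and triangle winding for all or one target triangle, using a custom stepped-loop macro.
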(event EventBeginPlay)

(event Collision|EventActorBeginOverlap
  (params (OtherActor :type Actor%20Object%20Reference)))

(event EventTick
  (params (DeltaSeconds :type Float%20%28single-precision%29)))

(fn ConstructionScript
  (CallFunction|DrawMesh)
  (if (Variables|Debug|GetDebug)
    (Rendering|Material|SetMaterial (Variables|Default|GetProceduralMesh) 0 (Utilities|Select :Index (Variables|Debug|GetMaterialType) :NewEnumerator0 "/Game/BluePrints/ProceduralModering/M_Procedural_Standard.M_Procedural_Standard" :NewEnumerator1 "/Game/BluePrints/ProceduralModering/M_Procedural_UV.M_Procedural_UV" :NewEnumerator2 "/Game/BluePrints/ProceduralModering/M_Procedural_Normal.M_Procedural_Normal"))
    (Debug|DrawVerticies)
    (Debug|DrawNormals)
    (Debug|DrawTrianglesArrow)))

(fn DrawMesh
  (return true))

(fn ClearArrays
  (Utilities|Array|Clear (Variables|Default|GetVeticies))
  (Utilities|Array|Clear (Variables|Default|GetNormals))
  (Utilities|Array|Clear (Variables|Default|GetUV))
  (Utilities|Array|Clear (Variables|Default|GetTriangles)))

(fn DrawNormals
  (for (_array_element _array_index) (Variables|Default|GetNormals)
    (AddComponent|AddArrowComponent false (Math|Transform|MakeTransform (Utilities|Array|Get(acopy) (Variables|Default|GetVeticies) _array_index) (Math|Conversions|RotationFromXVector _array_element) "0.100000,0.100000,0.100000"))))

(fn DrawVerticies
  (bind _veticies (Variables|Default|GetVeticies))
  (for (_array_element _array_index) _veticies
    (bind _returnvalue (AddComponent|AddStaticMeshComponent false (Math|Transform|MakeTransform _array_element "0, 0, 0" "0.050000,0.050000,0.050000")))
    (Rendering|Material|SetVectorParameterValueonMaterials _returnvalue "Color" (Math|Conversions|ToVector(Float) (/ (Math|Conversions|ToFloat(Integer) _array_index) (Math|Conversions|ToFloat(Integer) (Utilities|Array|Length _veticies)))))))

(fn DrawTrianglesArrow
  (bind _triangles (Variables|Default|GetTriangles))
  (bind _veticies (Variables|Default|GetVeticies))
  (bind _index (Utilities|ForLoopwithSelfCounter 0 (- (Utilities|Array|Length (Variables|Default|GetTriangles)) 2) 3)
    (:LoopBody
      (if (Variables|Debug|GetDrawTargetNumTriangle)
        (if (== _index (* (Variables|Debug|GetTargetNum) 3))
          (for (_array_element _array_index) (Utilities|Array|MakeArray (Utilities|Array|Get(acopy) _veticies (Utilities|Array|Get(acopy) _triangles _index)) (Utilities|Array|Get(acopy) _veticies (Utilities|Array|Get(acopy) _triangles (+ _index 1))) (Utilities|Array|Get(acopy) _veticies (Utilities|Array|Get(acopy) _triangles (+ _index 2)))) :!label _label
            (bind _returnvalue (AddComponent|AddArrowComponent false (Math|Transform|MakeTransform _array_element (Math|Rotator|FindLookatRotation _array_element (Utilities|Array|Get(acopy) (Utilities|Array|MakeArray (Utilities|Array|Get(acopy) _veticies (Utilities|Array|Get(acopy) _triangles _index)) (Utilities|Array|Get(acopy) _veticies (Utilities|Array|Get(acopy) _triangles (+ _index 1))) (Utilities|Array|Get(acopy) _veticies (Utilities|Array|Get(acopy) _triangles (+ _index 2)))) (Math|Integer|%(Integer) (+ _array_index 1) (Utilities|Array|Length (Utilities|Array|MakeArray (Utilities|Array|Get(acopy) _veticies (Utilities|Array|Get(acopy) _triangles _index)) (Utilities|Array|Get(acopy) _veticies (Utilities|Array|Get(acopy) _triangles (+ _index 1))) (Utilities|Array|Get(acopy) _veticies (Utilities|Array|Get(acopy) _triangles (+ _index 2)))))))) (Math|Vector|MakeVector (/ (Math|Vector|VectorLength (- _array_element (Utilities|Array|Get(acopy) (Utilities|Array|MakeArray (Utilities|Array|Get(acopy) _veticies (Utilities|Array|Get(acopy) _triangles _index)) (Utilities|Array|Get(acopy) _veticies (Utilities|Array|Get(acopy) _triangles (+ _index 1))) (Utilities|Array|Get(acopy) _veticies (Utilities|Array|Get(acopy) _triangles (+ _index 2)))) (Math|Integer|%(Integer) (+ _array_index 1) (Utilities|Array|Length (Utilities|Array|MakeArray (Utilities|Array|Get(acopy) _veticies (Utilities|Array|Get(acopy) _triangles _index)) (Utilities|Array|Get(acopy) _veticies (Utilities|Array|Get(acopy) _triangles (+ _index 1))) (Utilities|Array|Get(acopy) _veticies (Utilities|Array|Get(acopy) _triangles (+ _index 2))))))))) 75.0) 0.25 0.25))))
            (Components|Arrow|SetArrowColor(LinearColor) _returnvalue (Math|Color|SelectColor (Utilities|Select :Index _array_index :Option%200 "(R=0.980392,G=0.180392,B=0.400000,A=1.000000)" :Option%201 "(R=0.019608,G=0.603922,B=0.988235,A=1.000000)" :Option%202 "(R=1.000000,G=0.937255,B=0.090196,A=1.000000)") "(R=0.195485,G=0.940257,B=1.000000,A=1.000000)" (Variables|Debug|GetColorfulMode)))))
        (else
          (goto _label))))))