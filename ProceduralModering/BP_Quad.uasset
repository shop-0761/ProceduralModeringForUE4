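; BP_Quad is a procedural mesh Blueprint that builds a flat, upward-facing square centered on its origin.
; DrawMesh derives four corner vertices from Size and creates a ProceduralMesh section from two triangles with up normals and full 0–1 UVs.
; The construction script only calls its parent and the event graph is empty, so nothing in this graph calls DrawMesh directly.
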(event EventBeginPlay)

(event Collision|EventActorBeginOverlap
  (params (OtherActor :type Actor%20Object%20Reference)))

(event EventTick
  (params (DeltaSeconds :type Float%20%28single-precision%29)))

(fn ConstructionScript
  (|CallParentFunction))

(fn DrawMesh
  (bind _size (Variables|Default|GetSize))
  (bind _returnvalue (/ _size 2.0))
  (bind _returnvalue_2 (* _returnvalue -1.0))
  (bind _output_get (Variables|Default|SetVeticies (Utilities|Array|MakeArray (Math|Vector|MakeVector _returnvalue_2 _returnvalue 0.0) (Math|Vector|MakeVector _returnvalue _returnvalue 0.0) (Math|Vector|MakeVector _returnvalue _returnvalue_2 0.0) (Math|Vector|MakeVector _returnvalue_2 _returnvalue_2 0.0))))
  (bind _output_get_2 (Variables|Default|SetTriangles (Utilities|Array|MakeArray 0 1 2 2 3 0)))
  (bind _output_get_3 (Variables|Default|SetNormals (Utilities|Array|MakeArray "0, 0,1.000000" "0, 0,1.000000" "0.000000,0.000000,1.000000" "0.000000,0.000000,1.000000")))
  (bind _output_get_4 (Variables|Default|SetUV (Utilities|Array|MakeArray "" "(X=1.000000,Y=0.000000)" "(X=1.000000,Y=1.000000)" "(X=0.000000,Y=1.000000)")))
  (Class|ProceduralMeshComponent|CreateMeshSectionLinearColor (Variables|Default|GetProceduralMesh) 0 _output_get _output_get_2 _output_get_3 _output_get_4 0 0 false))