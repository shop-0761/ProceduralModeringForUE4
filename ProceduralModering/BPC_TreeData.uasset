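; Blueprint component that holds tree-shape parameters for procedural modeling and supplies randomized values from them.
; Three getters return a branch count, a growth angle within its min/max, and a bend symmetric around zero.
; The branch count's inclusive upper bound is BranchMax plus one, so it can exceed BranchMax.
; Results are unseeded, as the RandomSeed stream variants sit unconnected and the event graph is empty.
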(event EventBeginPlay)

(event EventTick
  (params (DeltaSeconds :type Float%20%28single-precision%29)))

(fn GetRandomBranches
  (return (Math|Random|RandomIntegerinRange (Variables|Default|GetBranchMin) (+ (Variables|Default|GetBranchMax) 1))))

(fn GetRandomGrowthAngle
  (return (Math|Random|RandomFloatinRange (Variables|Default|GetGrowAngleMin) (Variables|Default|GetGrowAngleMax))))

(fn GetRandomBendDegree
  (bind _benddegree (Variables|Default|GetBendDegree))
  (return (Math|Random|RandomFloatinRange (* _benddegree -1.0) _benddegree)))