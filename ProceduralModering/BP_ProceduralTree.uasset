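; Procedural tree actor that builds a branching tree as one procedural mesh, with a selectable standard, UV or normal material.
; DrawMesh spawns a root BP_TreeBranch, measures the longest branch path, then recursively walks the children.
; Each branch's segment frames become tube rings and triangles, with V coordinates normalized by that path length.
; The branch actors serve only as temporary data and are destroyed before the mesh section is created.
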(event EventBeginPlay
  (|CallParentFunction)
  (Rendering|Material|SetMaterial (Variables|Default|GetProceduralMesh) 0 (Utilities|Select :Index (Variables|Default|GetMaterialType) :NewEnumerator0 "/Game/BluePrints/ProceduralModering/M_Procedural_Standard.M_Procedural_Standard" :NewEnumerator1 "/Game/BluePrints/ProceduralModering/M_Procedural_UV.M_Procedural_UV" :NewEnumerator2 "/Game/BluePrints/ProceduralModering/M_Procedural_Normal.M_Procedural_Normal")))

(event Collision|EventActorBeginOverlap
  (params (OtherActor :type Actor%20Object%20Reference)))

(event EventTick
  (params (DeltaSeconds :type Float%20%28single-precision%29)))

(event EventClearArrays
  (Utilities|Array|Clear (Variables|Default|GetVeticies))
  (Utilities|Array|Clear (Variables|Default|GetNormals))
  (Utilities|Array|Clear (Variables|Default|GetUV))
  (Utilities|Array|Clear (Variables|Default|GetTriangles))
  (Utilities|Array|Clear (Variables|Default|GetTangents)))

(fn ConstructionScript)

(fn DrawMesh
  (bind _generations (Variables|Default|GetGenerations))
  (bind _returnvalue (Game|SpawnActorfromClass "/Game/BluePrints/ProceduralModering/BP_TreeBranch.BP_TreeBranch_C" (Transformation|GetActorTransform) "Undefined" 0 _generations _generations "0.000000,0.000000,0.000000" (Utilities|Struct|MakeProcMeshTangent (Transformation|GetActorUpVector) false) (Transformation|GetActorForwardVector) (* (Transformation|GetActorRightVector) -1.0) (Variables|Default|GetLength) (Variables|Default|GetRadius) 0.0 (Variables|Default|GetBPC_TreeData)))
  (bind _output_get (LocalVariables|Set_Root _returnvalue))
  (Variables|Default|SetMaxLength (CallFunction|TraverseMaxLength _output_get))
  (CallFunction|Traverse _output_get)
  (CallFunction|DestroyBranches _output_get)
  (Class|ProceduralMeshComponent|CreateMeshSectionLinearColor (Variables|Default|GetProceduralMesh) 0 (Variables|Default|GetVeticies) (Variables|Default|GetTriangles) (Variables|Default|GetNormals) (Variables|Default|GetUV) 0 (Variables|Default|GetTangents) false)
  (return true))

(fn TraverseMaxLength
  (params (Branch :type BP%20Tree%20Branch%20Object%20Reference))
  (LocalVariables|Set_Max 0.0)
  (for _array_element (Variables|/Game/BluePrints/ProceduralModering/BP_TreeBranch.BP_TreeBranch_C|GetBranchChildren Branch)
    (LocalVariables|Set_Max (Math|Float|Max(Float) (LocalVariables|Get_Max) (CallFunction|TraverseMaxLength _array_element))))
  (return (+ (Variables|/Game/BluePrints/ProceduralModering/BP_TreeBranch.BP_TreeBranch_C|GetLength Branch) (LocalVariables|Get_Max))))

(fn Traverse
  (params (From :type BP%20Tree%20Branch%20Object%20Reference))
  (bind _branchchildren (Variables|/Game/BluePrints/ProceduralModering/BP_TreeBranch.BP_TreeBranch_C|GetBranchChildren From))
  (if (> (Utilities|Array|Length _branchchildren) 0)
    (for _array_element _branchchildren
      (CallFunction|Traverse _array_element)))
  (CallFunction|TraverseCallBack From))

(fn TraverseCallBack
  (params (Branch :type BP%20Tree%20Branch%20Object%20Reference))
  (bind _segments (Variables|/Game/BluePrints/ProceduralModering/BP_TreeBranch.BP_TreeBranch_C|GetSegments Branch))
  (bind _bpc_treedata (Variables|Default|GetBPC_TreeData))
  (bind _bpc_treedata_2 (Variables|Default|GetBPC_TreeData))
  (bind _radialsegments (Variables|/Game/BluePrints/ProceduralModering/BPC_TreeData.BPC_TreeData_C|GetRadialSegments _bpc_treedata))
  (bind _radialsegments_2 (Variables|/Game/BluePrints/ProceduralModering/BPC_TreeData.BPC_TreeData_C|GetRadialSegments _bpc_treedata_2))
  (bind _returnvalue (+ _radialsegments_2 1))
  (LocalVariables|Set_Offset (Utilities|Array|Length (Variables|Default|GetVeticies)))
  (LocalVariables|Set_VOffset (/ (Variables|/Game/BluePrints/ProceduralModering/BP_TreeBranch.BP_TreeBranch_C|GetOffset Branch) (Variables|Default|GetMaxLength)))
  (LocalVariables|Set_VLength (/ (Variables|/Game/BluePrints/ProceduralModering/BP_TreeBranch.BP_TreeBranch_C|GetLength Branch) (Variables|Default|GetMaxLength)))
  (for (_array_element _array_index) _segments
    (LocalVariables|Set_V (+ (LocalVariables|Get_VOffset) (* (/ (Math|Conversions|ToFloat(Integer) _array_index) (Math|Conversions|ToFloat(Integer) (- (Utilities|Array|Length _segments) 1))) (LocalVariables|Get_VLength))))
    (for _index (range 0 (+ _radialsegments 1))
      (Utilities|Array|Add (Variables|Default|GetVeticies) (+ (.Location (Utilities|Struct|BreakTreeSegment _array_element)) (* (Math|Vector|Normalize (+ (* (.Normal (Utilities|Struct|BreakFrenetFrame (.Frame (Utilities|Struct|BreakTreeSegment _array_element)))) (Math|Trig|Cos(Radians) (* (/ (Math|Conversions|ToFloat(Integer) _index) (Math|Conversions|ToFloat(Integer) _radialsegments)) (* (Math|Trig|GetPI) 2.0)))) (* (.Binormal (Utilities|Struct|BreakFrenetFrame (.Frame (Utilities|Struct|BreakTreeSegment _array_element)))) (Math|Trig|Sin(Radians) (* (/ (Math|Conversions|ToFloat(Integer) _index) (Math|Conversions|ToFloat(Integer) _radialsegments)) (* (Math|Trig|GetPI) 2.0)))))) (.Radius (Utilities|Struct|BreakTreeSegment _array_element)))))
      (Utilities|Array|Add (Variables|Default|GetNormals) (Math|Vector|Normalize (+ (* (.Normal (Utilities|Struct|BreakFrenetFrame (.Frame (Utilities|Struct|BreakTreeSegment _array_element)))) (Math|Trig|Cos(Radians) (* (/ (Math|Conversions|ToFloat(Integer) _index) (Math|Conversions|ToFloat(Integer) _radialsegments)) (* (Math|Trig|GetPI) 2.0)))) (* (.Binormal (Utilities|Struct|BreakFrenetFrame (.Frame (Utilities|Struct|BreakTreeSegment _array_element)))) (Math|Trig|Sin(Radians) (* (/ (Math|Conversions|ToFloat(Integer) _index) (Math|Conversions|ToFloat(Integer) _radialsegments)) (* (Math|Trig|GetPI) 2.0)))))))
      (Utilities|Array|Add (Variables|Default|GetTangents) (.Tangent (Utilities|Struct|BreakFrenetFrame (.Frame (Utilities|Struct|BreakTreeSegment _array_element)))))
      (Utilities|Array|Add (Variables|Default|GetUV) (Math|Vector2D|MakeVector2D (/ (Math|Conversions|ToFloat(Integer) _index) (Math|Conversions|ToFloat(Integer) _radialsegments)) (LocalVariables|Get_V)))))
  (for _index_2 (range 1 (+ (Variables|/Game/BluePrints/ProceduralModering/BPC_TreeData.BPC_TreeData_C|GetHeightSegments _bpc_treedata_2) 1)) ; j
    (for _index_3 (range 1 _returnvalue) ; i
      (LocalVariables|Set_a (+ (+ (- _index_3 1) (* (- _index_2 1) _returnvalue)) (LocalVariables|Get_Offset)))
      (LocalVariables|Set_b (+ (LocalVariables|Get_Offset) (+ (- _index_3 1) (* _index_2 _returnvalue))))
      (LocalVariables|Set_c (+ (LocalVariables|Get_Offset) (+ _index_3 (* _index_2 _returnvalue))))
      (LocalVariables|Set_d (+ (LocalVariables|Get_Offset) (+ (* (- _index_2 1) _returnvalue) _index_3)))
      (Utilities|Array|AppendArray (Variables|Default|GetTriangles) (Utilities|Array|MakeArray (LocalVariables|Get_a) (LocalVariables|Get_d) (LocalVariables|Get_b) (LocalVariables|Get_b) (LocalVariables|Get_d) (LocalVariables|Get_c))))))

(fn DestroyBranches
  (params (Root :type BP%20Tree%20Branch%20Object%20Reference))
  (bind _branchchildren (Variables|/Game/BluePrints/ProceduralModering/BP_TreeBranch.BP_TreeBranch_C|GetBranchChildren Root))
  (if (> (Utilities|Array|Length _branchchildren) 0)
    (for _array_element _branchchildren
      (CallFunction|DestroyBranches _array_element)))
  (Actor|DestroyActor Root))