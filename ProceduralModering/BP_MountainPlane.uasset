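; BP_MountainPlane is a procedural modeling Blueprint that defines a mountain-shaped height profile for a plane.
; DepthFunc multiplies the Distance falloff of Rx and Ry by Depth, giving a peak at the center of the 0–1 range that drops to zero at the edges.
; Distance folds its input around the midpoint and raises it to Power to shape the slope.
; The construction script only calls its parent, and the event graph is empty.
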(event EventBeginPlay)

(event Collision|EventActorBeginOverlap
  (params (OtherActor :type Actor%20Object%20Reference)))

(event EventTick
  (params (DeltaSeconds :type Float%20%28single-precision%29)))

(fn ConstructionScript
  (|CallParentFunction))

(fn Distance
  (params (v :type Float%20%28single-precision%29))
  (return (Math|Float|Power (- 0.5 (Math|Float|Absolute(Float) (- 0.5 v))) (Variables|Default|GetPower))))

(fn DepthFunc
  (params (rx :type Float%20%28single-precision%29) (ry :type Float%20%28single-precision%29))
  (return (* (CallFunction|Distance rx) (CallFunction|Distance ry) (Variables|Default|GetDepth))))